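; Gear road module placeable (D5 variant) that plays a material-driven build animation on its road mesh.
; PlayBuildAnim passes RoadBuildMesh to a helper event, which creates a dynamic material instance on slot 0 of each mesh it receives.
; The helper stamps the current game time as the animation start and sets the inversion parameter from MirrorX, leaving the animation to the material.
; Construction only calls the parent script.
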(event Custom|CustomEvent
  (params (NewParam :type Array%20of%20Static%20Mesh%20Component%20Object%20References))
  (for _array_element NewParam
    (bind _returnvalue (Rendering|Material|CreateDynamicMaterialInstance _array_element 0 0 "None" :!class /Script/Engine.PrimitiveComponent))
    (Rendering|Material|SetScalarParameterValue _returnvalue "BuildAnimStartTime" (Utilities|Time|GetTimeSeconds) :!class /Script/Engine.MaterialInstanceDynamic)
    (Rendering|Material|SetScalarParameterValue _returnvalue "BuildInverted" (Math|Conversions|ToFloat(Boolean) (Variables|Default|GetbMirrorX)) :!class /Script/Engine.MaterialInstanceDynamic)))

(event EventBeginPlay)

(event Collision|EventActorBeginOverlap
  (params (OtherActor :type Actor%20Object%20Reference)))

(event EventTick
  (params (DeltaSeconds :type Float%20%28single-precision%29)))

(event EventPlayBuildAnim
  (CallFunction|CustomEvent (Utilities|Array|MakeArray (Variables|Default|GetRoadBuildMesh))))

(fn ConstructionScript
  (|CallParentFunction))