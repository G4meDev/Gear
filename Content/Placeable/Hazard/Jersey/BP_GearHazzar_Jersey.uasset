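; BP_GearHazzar_Jersey is a placeable hazard, named as a Jersey barrier, whose main mesh becomes a solid obstacle when enabled.
; Idle shows the mesh without collision, Enabled shows it blocking everything, and leaving either state hides it and disables collision.
; Start and end functions for both states route through shared helpers that swap the collision profile and toggle in-game visibility.
; It reports hazard bounds from the mesh's local bounds.
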(event EventBeginPlay
  (|CallParentFunction) ; This node is disabled and will not be called.\nDrag off pins to build functionality.
)

(event Collision|EventActorBeginOverlap
  (params (OtherActor :type Actor%20Object%20Reference))
  (|CallParentFunction OtherActor) ; This node is disabled and will not be called.\nDrag off pins to build functionality.
)

(event EventTick
  (params (DeltaSeconds :type Float%20%28single-precision%29))
  (|CallParentFunction DeltaSeconds) ; This node is disabled and will not be called.\nDrag off pins to build functionality.
)

(fn ConstructionScript
  (|CallParentFunction))

(fn GetHazardBounds
  (bind _mainmesh (Variables|Default|GetMainMesh))
  (bind (_min _max) (Components|StaticMesh|GetLocalBounds _mainmesh))
  (return _min _max))

(fn IdleStart
  (CallFunction|SetCollisionsEnabled false)
  (CallFunction|SetVisible true)
  (return))

(fn IdleEnd
  (CallFunction|SetCollisionsEnabled false)
  (CallFunction|SetVisible false)
  (return))

(fn EnabledStart
  (CallFunction|SetCollisionsEnabled true)
  (CallFunction|SetVisible true)
  (return))

(fn EnabledEnd
  (CallFunction|SetCollisionsEnabled false)
  (CallFunction|SetVisible false)
  (return))

(fn SetCollisionsEnabled
  (params (Enabled :type Boolean))
  (Collision|SetCollisionProfileName (Variables|Default|GetMainMesh) (Utilities|String|SelectName "BlockAll" "NoCollision" Enabled) true :!class /Script/Engine.PrimitiveComponent)
  (return))

(fn SetVisible
  (params (Visible :type Boolean))
  (Development|SetHiddeninGame (Variables|Default|GetMainMesh) (not Visible) false)
  (return))