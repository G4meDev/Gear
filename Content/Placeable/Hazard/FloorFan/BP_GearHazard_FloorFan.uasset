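; Placeable floor fan hazard that pushes overlapping GearVehicles upward while in the Enabled state.
; MainMesh overlap events maintain the vehicle list, and Tick applies ForceStrength along world up to each vehicle's mesh.
; Idle and Enabled state functions toggle mesh visibility and its vehicle-only trigger collision profile.
; BeginPlay and Enabled start both activate collision, play the fan sound and clear the vehicle list.
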(event OnComponentBeginOverlap(MainMesh)
  (params (OverlappedComponent :type Primitive%20Component%20Object%20Reference) (OtherActor :type Actor%20Object%20Reference) (OtherComp :type Primitive%20Component%20Object%20Reference) (OtherBodyIndex :type Integer) (bFromSweep :type Boolean) (SweepResult :type Hit%20Result%20Structure%20%28by%20ref%29))
  (bind _asgear_vehicle (Utilities|Casting|CastToGearVehicle OtherActor))
  (Utilities|Array|AddUnique (Variables|Default|GetOverlappingVehicles) _asgear_vehicle))

(event OnComponentEndOverlap(MainMesh)
  (params (OverlappedComponent :type Primitive%20Component%20Object%20Reference) (OtherActor :type Actor%20Object%20Reference) (OtherComp :type Primitive%20Component%20Object%20Reference) (OtherBodyIndex :type Integer))
  (bind _asgear_vehicle (Utilities|Casting|CastToGearVehicle OtherActor))
  (Utilities|Array|RemoveItem (Variables|Default|GetOverlappingVehicles) _asgear_vehicle))

(event EventBeginPlay
  (|CallParentFunction)
  (CallFunction|SetCollisionsEnabled true)
  (CallFunction|SetVisible true)
  (Audio|Components|Audio|Play (Variables|Default|GetSFX_FloorFan) 0.0)
  (Utilities|Array|Clear (Variables|Default|GetOverlappingVehicles)))

(event Collision|EventActorBeginOverlap
  (params (OtherActor :type Actor%20Object%20Reference))
  (|CallParentFunction OtherActor) ; This node is disabled and will not be called.\nDrag off pins to build functionality.
)

(event EventTick
  (params (DeltaSeconds :type Float%20%28single-precision%29))
  (|CallParentFunction DeltaSeconds)
  (if (Utilities|Enum|Equal(Enum) (Variables|Default|GetPlaceableState) "Enabled")
    (for _array_element (Variables|Default|GetOverlappingVehicles)
      (Utilities|IsValid _array_element
        (:Is%20Valid
          (Physics|AddForce (Variables|/Script/ChaosVehicles.WheeledVehiclePawn|GetMesh _array_element) (* (Math|Vector|VectorUp) (Variables|Default|GetForceStrength)) "None" false))))))

(fn ConstructionScript
  (|CallParentFunction))

(fn GetHazardBounds
  (bind _mainmesh (Variables|Default|GetMainMesh))
  (bind (_min _max) (Components|StaticMesh|GetLocalBounds _mainmesh))
  (return _min _max))

(fn IdleStart
  (CallFunction|SetCollisionsEnabled false)
  (CallFunction|SetVisible true)
  (return))

(fn IdleEnd
  (CallFunction|SetCollisionsEnabled false)
  (CallFunction|SetVisible false)
  (return))

(fn EnabledStart
  (CallFunction|SetCollisionsEnabled true)
  (CallFunction|SetVisible true)
  (Audio|Components|Audio|Play (Variables|Default|GetSFX_FloorFan) 0.0)
  (Utilities|Array|Clear (Variables|Default|GetOverlappingVehicles))
  (return))

(fn EnabledEnd
  (CallFunction|SetCollisionsEnabled false)
  (CallFunction|SetVisible false)
  (return))

(fn SetCollisionsEnabled
  (params (Enabled :type Boolean))
  (Collision|SetCollisionProfileName (Variables|Default|GetMainMesh) (Utilities|String|SelectName "TriggerOnlyVehicle" "NoCollision" Enabled) true :!class /Script/Engine.PrimitiveComponent)
  (return))

(fn SetVisible
  (params (Visible :type Boolean))
  (Development|SetHiddeninGame (Variables|Default|GetMainMesh) (not Visible) false)
  (return))