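; BP_GearHazzar_Itembox is a placeable hazard actor that groups four item boxes into one piece.
; On BeginPlay it initializes each Itembox with its own mesh and hitbox.
; Its idle and enabled start and end functions simply forward each state change to all four boxes.
; GetHazardBounds returns zero bounds.
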(event EventBeginPlay
  (|CallParentFunction)
  (CallFunction|InitItems))

(event Collision|EventActorBeginOverlap
  (params (OtherActor :type Actor%20Object%20Reference))
  (|CallParentFunction OtherActor) ; This node is disabled and will not be called.\nDrag off pins to build functionality.
)

(event EventTick
  (params (DeltaSeconds :type Float%20%28single-precision%29))
  (|CallParentFunction DeltaSeconds) ; This node is disabled and will not be called.\nDrag off pins to build functionality.
)

(fn ConstructionScript
  (|CallParentFunction))

(fn GetHazardBounds
  (return "0, 0, 0" "0, 0, 0"))

(fn IdleStart
  (Default|IdleStart (Variables|Default|GetItembox_1))
  (return))

(fn IdleEnd
  (Default|IdleEnd (Variables|Default|GetItembox_1))
  (return))

(fn EnabledStart
  (Default|EnabledStart (Variables|Default|GetItembox_1))
  (return))

(fn EnabledEnd
  (Default|EnabledEnd (Variables|Default|GetItembox_1))
  (return))

(fn InitItems
  (Default|InitItembox (Variables|Default|GetItembox_1) (Variables|Default|GetMesh_1) (Variables|Default|GetHitbox_1))
  (Default|InitItembox (Variables|Default|GetItembox_2) (Variables|Default|GetMesh_2) (Variables|Default|GetHitbox_2))
  (Default|InitItembox (Variables|Default|GetItembox_3) (Variables|Default|GetMesh_3) (Variables|Default|GetHitbox_3))
  (Default|InitItembox (Variables|Default|GetItembox_4) (Variables|Default|GetMesh_4) (Variables|Default|GetHitbox_4))
  (return))