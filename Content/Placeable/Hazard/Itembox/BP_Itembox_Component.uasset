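; Itembox component that gives a random ability to a vehicle driving into it.
; InitItembox receives the mesh and collision components and binds the overlap event.
; Idle and Enabled start/end functions toggle visibility and a vehicle-only trigger profile, which is active only with authority.
; On an authoritative overlap, a GearVehicle without an ability gets one from GearGameMode, then the box hides and disables collision.
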(event Custom|ItemGrabed
  (CallFunction|SetVisible false))

(event EventBeginPlay)

(event EventTick
  (params (DeltaSeconds :type Float%20%28single-precision%29)))

(fn InitItembox
  (params (Mesh :type Static%20Mesh%20Component%20Object%20Reference) (Collision :type Sphere%20Component%20Object%20Reference))
  (Variables|Default|SetMeshComponent Mesh)
  (bind _output_get (Variables|Default|SetCollisionComponenet Collision))
  (Collision|BindEventtoOnComponentBeginOverlap _output_get (EventDispatchers|CreateEvent :!event OnBeginOverlap))
  (return))

(fn SetVisible
  (params (Visibility :type Boolean))
  (bind _meshcomponent (Variables|Default|GetMeshComponent)
    (:then
      (Development|SetHiddeninGame _meshcomponent (not Visibility) false)
      (return))
    (:else
      (return))))

(fn SetCollisionEnabled
  (params (Enabled :type Boolean))
  (bind _collisioncomponenet (Variables|Default|GetCollisionComponenet)
    (:then
      (Collision|SetCollisionProfileName _collisioncomponenet (Utilities|String|SelectName "TriggerOnlyVehicle" "NoCollision" (and Enabled (Ability|HasAuthority (Components|GetOwner)))) true :!class /Script/Engine.PrimitiveComponent)
      (return))
    (:else
      (return))))

(fn IdleStart
  (CallFunction|SetVisible true)
  (CallFunction|SetCollisionEnabled false)
  (return))

(fn IdleEnd
  (CallFunction|SetVisible false)
  (CallFunction|SetCollisionEnabled false)
  (return))

(fn EnabledStart
  (CallFunction|SetVisible true)
  (CallFunction|SetCollisionEnabled true)
  (return))

(fn EnabledEnd
  (CallFunction|SetVisible false)
  (CallFunction|SetCollisionEnabled false)
  (return))

(fn OnBeginOverlap
  (params (OverlappedComponent :type Primitive%20Component%20Object%20Reference) (OtherActor :type Actor%20Object%20Reference) (OtherComp :type Primitive%20Component%20Object%20Reference) (OtherBodyIndex :type Integer) (bFromSweep :type Boolean) (SweepResult :type Hit%20Result%20Structure%20%28by%20ref%29))
  (if (Ability|HasAuthority (Components|GetOwner))
    (Utilities|FlowControl|Sequence
      (:then_0
        (bind _asgear_vehicle (Utilities|Casting|CastToGearVehicle OtherActor))
        (if (not (Class|GearVehicle|HasAbility _asgear_vehicle))
          (bind _asgear_game_mode (Utilities|Casting|CastToGearGameMode (Game|GetGameMode)))
          (Class|GearVehicle|GrantAbility _asgear_vehicle (Class|GearGameMode|GetRandomAbility _asgear_game_mode))
          (CallFunction|SetCollisionEnabled false)
          (CallFunction|ItemGrabed)
          (return)))
      (:then_1
        (Development|PrintString (Utilities|String|Append (Utilities|GetDisplayName OtherActor) " hit : " (Utilities|GetDisplayName self)) false)))))