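; BP_GearDriver_Tricycle is a tricycle driver actor with separate body and head meshes, where the head uses physical animation.
; On BeginPlay it applies profile "D" below head_002 and simulates physics on that bone chain.
; Tick caches the body's world-space head bone transform in HeadTransform, which this graph never reads.
; An item-grab montage test event exists, but its looping timer setup is disconnected.
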(event Custom|CustomEvent
  (Development|PrintString "Hello")
  (Animation|Montage|PlayMontage (Variables|Default|GetBodyMesh) "/Game/Driver/NewFolder/AM_ItemGrab.AM_ItemGrab"))

(event EventBeginPlay
  (bind _returnvalue (Utilities|Name|MakeLiteralName "head_002"))
  (bind _headphysicalanimation (Variables|Default|GetHeadPhysicalAnimation))
  (bind _headmesh (Variables|Default|GetHeadMesh))
  (Class|PhysicalAnimationComponent|SetSkeletalMeshComponent _headphysicalanimation _headmesh)
  (Class|PhysicalAnimationComponent|ApplyPhysicalAnimationProfileBelow _headphysicalanimation _returnvalue "D" true false)
  (Class|SkeletalMeshComponent|SetAllBodiesBelowSimulatePhysics _headmesh _returnvalue true true))

(event Collision|EventActorBeginOverlap
  (params (OtherActor :type Actor%20Object%20Reference)))

(event EventTick
  (params (DeltaSeconds :type Float%20%28single-precision%29))
  (Variables|Default|SetHeadTransform (Transformation|GetBoneTransform (Variables|Default|GetBodyMesh) "head" "RTS_World")))

(fn ConstructionScript)