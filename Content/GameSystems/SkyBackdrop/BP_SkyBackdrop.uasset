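; Sky backdrop actor that periodically spawns BP_Airplane actors at cloud height around the player's view.
; A randomized timer calls SpawnPlane, which re-arms it whether or not a plane spawns.
; SpawnPlane intersects the player's view with a horizontal plane at CloudHeight from MPC_WorldParameters.
; If that hits, the airplane spawns at a random horizontal offset within PlaneSpawnRadius, rotated to face the intersection point.
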(event EventBeginPlay
  (CallFunction|SetNextPlaneTimer))

(event Collision|EventActorBeginOverlap
  (params (OtherActor :type Actor%20Object%20Reference)))

(event EventTick
  (params (DeltaSeconds :type Float%20%28single-precision%29)))

(fn ConstructionScript)

(fn SpawnPlane
  (bind _planespawnradius (Variables|Default|GetPlaneSpawnRadius))
  (Utilities|FlowControl|Sequence
    (:then_0
      (bind _returnvalue (Rendering|Material|GetScalarParameterValue "/Game/Common/Material/Collection/MPC_WorldParameters.MPC_WorldParameters" "CloudHeight" :!class /Script/Engine.KismetMaterialLibrary))
      (if (.ReturnValue (Class|GearStatics|GetPlayerViewZPlaneIntersection (Game|GetPlayerController 0) _returnvalue))
        (Game|SpawnActorfromClass "/Game/GameSystems/Airplane/BP_Airplane.BP_Airplane_C" (Math|Transform|MakeTransform (+ (.Result (Class|GearStatics|GetPlayerViewZPlaneIntersection (Game|GetPlayerController 0) _returnvalue)) (* (Math|Random|RandomUnitVector) (Math|Vector|MakeVector _planespawnradius _planespawnradius 0.0))) (Math|Rotator|FindLookatRotation (+ (.Result (Class|GearStatics|GetPlayerViewZPlaneIntersection (Game|GetPlayerController 0) _returnvalue)) (* (Math|Random|RandomUnitVector) (Math|Vector|MakeVector _planespawnradius _planespawnradius 0.0))) (.Result (Class|GearStatics|GetPlayerViewZPlaneIntersection (Game|GetPlayerController 0) _returnvalue)))) "Undefined" "MultiplyWithRoot" 0 0)))
    (:then_1
      (CallFunction|SetNextPlaneTimer))))

(fn SetNextPlaneTimer
  (Utilities|Time|SetTimerbyFunctionName 0 "SpawnPlane" (Math|Random|RandomFloatinRange (Variables|Default|GetPlaneSpawnMinTime) (Variables|Default|GetPlaneSpawnMaxTime)))
  (return))