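; BP_Airplane is a short-lived airplane actor that flies straight ahead at a set speed and fades through its lifetime.
; Tick moves it along its forward vector and drives the material's Opacity from a float curve sampled at normalized age.
; When Lifetime ends, it hides the mesh and deactivates both wing effects, then lingers for WingLifeTime before destruction so the effects can die out.
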(event Custom|MarkDead
  (Variables|Default|SetAlive false)
  (Rendering|SetVisibility (Variables|Default|GetStaticMesh) false false)
  (Components|Activation|Deactivate (Variables|Default|GetFX_AirplaneWing1)))

(event EventBeginPlay
  (Utilities|Time|SetTimerbyEvent (delegate Custom|MarkDead) (Variables|Default|GetLifetime))
  (Actor|SetLifeSpan (+ (Variables|Default|GetLifetime) (Variables|Default|GetWingLifeTime)))
  (Variables|Default|SetStartTime (Utilities|Time|GetTimeSeconds))
  (bind _returnvalue (Rendering|Material|CreateDynamicMaterialInstance (Variables|Default|GetStaticMesh) 0 0 "None" :!class /Script/Engine.PrimitiveComponent))
  (Variables|Default|SetPlaneMaterial _returnvalue))

(event EventTick
  (params (DeltaSeconds :type Float%20%28single-precision%29))
  (if (Variables|Default|GetAlive)
    (Transformation|SetActorLocation (+ (Transformation|GetActorLocation) (* DeltaSeconds (Transformation|GetActorForwardVector) (Variables|Default|GetSpeed))) false false)
    (Variables|Default|SetRelativeLifeTime (/ (- (Utilities|Time|GetTimeSeconds) (Variables|Default|GetStartTime)) (Variables|Default|GetLifetime)))
    (Rendering|Material|SetScalarParameterValue (Variables|Default|GetPlaneMaterial) "Opacity" (Math|Curves|GetFloatValue (Variables|Default|GetPlaneOpacityCurve) (Variables|Default|GetRelativeLifeTime)) :!class /Script/Engine.MaterialInstanceDynamic)))

(fn ConstructionScript)