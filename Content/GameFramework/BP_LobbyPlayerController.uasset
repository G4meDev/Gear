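; Lobby player controller Blueprint that relays match start countdown events to the lobby menu UI.
; Start and cancel events cast the LobbyWidget to W_LobbyMenu and forward the call, including the start time.
; Player add and remove events call local AddPlayer and RemovePlayer functions, which are currently empty.
; Disconnected leftover nodes include a pass that adds every existing lobby player state on the local controller.
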(event EventBeginPlay
  (|CallParentFunction))

(event EventTick
  (params (DeltaSeconds :type Float%20%28single-precision%29)))

(event EventOnAddPlayer
  (params (InPlayer :type Lobby%20Player%20State%20Object%20Reference))
  (CallFunction|AddPlayer InPlayer))

(event EventOnRemovePlayer
  (params (InPlayer :type Lobby%20Player%20State%20Object%20Reference))
  (CallFunction|RemovePlayer InPlayer))

(event EventOnStartGame
  (params (StartTime :type Float%20%28single-precision%29))
  (bind _asw_lobby_menu (Utilities|Casting|CastToW_LobbyMenu (Variables|Default|GetLobbyWidget)))
  (Default|OnStartGame _asw_lobby_menu StartTime))

(event EventOnStartGameCancel
  (bind _asw_lobby_menu (Utilities|Casting|CastToW_LobbyMenu (Variables|Default|GetLobbyWidget)))
  (Default|OnStartGameCancel _asw_lobby_menu))

(fn ConstructionScript)

(fn AddPlayer
  (params (Player :type Lobby%20Player%20State%20Object%20Reference)))

(fn RemovePlayer
  (params (Player :type Lobby%20Player%20State%20Object%20Reference)))