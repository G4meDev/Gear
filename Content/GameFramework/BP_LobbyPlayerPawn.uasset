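; BP_LobbyPlayerPawn is the lobby pawn that turns screen input into rotation of the player platforms.
; On BeginPlay it gathers every BP_LobbyPlayerPlatform in the level into an array.
; The IA_MoveScreen Enhanced Input action passes its X value to Rotate on each platform, and IA_TouchEnd calls ClearGrabbed on all of them.
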(event Input|EnhancedActionEvents|EnhancedInputActionIA_MoveScreen
  (params (ActionValue :type Vector%202D%20Structure) (ElapsedSeconds :type Float%20%28double-precision%29) (TriggeredSeconds :type Float%20%28double-precision%29) (InputAction :type Input%20Action%20Object%20Reference :default "/Game/Input/IA_MoveScreen.IA_MoveScreen"))
  (for _array_element (Variables|Default|GetPlatforms)
    (Class|LobbyPlayerPlatform|Rotate _array_element (.X (Math|Vector2D|BreakVector2D ActionValue)))))

(event Input|EnhancedActionEvents|EnhancedInputActionIA_TouchEnd
  (params (ActionValue :type Float%20%28double-precision%29) (ElapsedSeconds :type Float%20%28double-precision%29) (TriggeredSeconds :type Float%20%28double-precision%29) (InputAction :type Input%20Action%20Object%20Reference :default "/Game/Input/IA_TouchEnd.IA_TouchEnd"))
  (for _array_element (Variables|Default|GetPlatforms)
    (Class|LobbyPlayerPlatform|ClearGrabbed _array_element)))

(event EventBeginPlay
  (bind _outactors (Actor|GetAllActorsOfClass "/Game/GameSystems/LobbyPlayerPlatform/BP_LobbyPlayerPlatform.BP_LobbyPlayerPlatform_C"))
  (Variables|Default|SetPlatforms _outactors))

(event Collision|EventActorBeginOverlap
  (params (OtherActor :type Actor%20Object%20Reference)))

(event EventTick
  (params (DeltaSeconds :type Float%20%28single-precision%29)))

(fn ConstructionScript)