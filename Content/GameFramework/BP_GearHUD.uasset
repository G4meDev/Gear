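; BP_GearHUD is a HUD Blueprint that manages the waiting screen shown while players join.
; ShowWaitingScreen creates a W_WaitingScreen widget, stores it and adds it to the viewport, and RemoveWaitingScreen removes it and clears the reference.
; AddPlayer, RemovePlayer and AllPlayersJoined forward to that widget when it is valid.
; The event graph and construction script hold no logic.
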(event EventBeginPlay)

(event Collision|EventActorBeginOverlap
  (params (OtherActor :type Actor%20Object%20Reference)))

(event EventTick
  (params (DeltaSeconds :type Float%20%28single-precision%29)))

(fn ConstructionScript)

(fn ShowWaitingScreen
  (bind _returnvalue (UserInterface|CreateWidget "/Game/UI/WaitingScreen/W_WaitingScreen.W_WaitingScreen_C"))
  (bind _output_get (Variables|Default|SetWaitingScreenWidget _returnvalue))
  (UserInterface|Viewport|AddtoViewport _output_get 0)
  (return))

(fn RemoveWaitingScreen
  (Utilities|IsValid (Variables|Default|GetWaitingScreenWidget)
    (:Is%20Valid
      (Widget|RemovefromParent (Variables|Default|GetWaitingScreenWidget))
      (Variables|Default|SetWaitingScreenWidget 0)
      (return))))

(fn AddPlayer
  (params (InPlayer :type Gear%20Player%20State%20Object%20Reference))
  (bind _waitingscreenwidget (Variables|Default|GetWaitingScreenWidget))
  (Utilities|IsValid _waitingscreenwidget
    (:Is%20Valid
      (Default|AddPlayer _waitingscreenwidget InPlayer)
      (return))))

(fn RemovePlayer
  (params (InPlayer :type Gear%20Player%20State%20Object%20Reference))
  (bind _waitingscreenwidget (Variables|Default|GetWaitingScreenWidget))
  (Utilities|IsValid _waitingscreenwidget
    (:Is%20Valid
      (Default|RemovePlayer _waitingscreenwidget InPlayer)
      (return))))

(fn AllPlayersJoined
  (bind _waitingscreenwidget (Variables|Default|GetWaitingScreenWidget))
  (Utilities|IsValid _waitingscreenwidget
    (:Is%20Valid
      (Default|AllPlayersJoined _waitingscreenwidget)
      (return))))