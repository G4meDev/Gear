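; Player controller Blueprint that shows a waiting screen listing the players in the game.
; On BeginPlay, only the local controller creates W_WaitingScreen, adds it to the viewport and fills it with every existing GearPlayerState.
; OnAddPlayer and OnRemovePlayer events then keep the widget in sync through helper functions that skip the update when the widget is invalid.
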(event EventBeginPlay
  (if (Pawn|IsLocalController)
    (Utilities|FlowControl|Sequence
      (:then_0
        (bind _returnvalue (UserInterface|CreateWidget "/Game/UI/WaitingScreen/W_WaitingScreen.W_WaitingScreen_C"))
        (bind _output_get (Variables|Default|SetWaitingScreenWidget _returnvalue))
        (UserInterface|Viewport|AddtoViewport _output_get 0))
      (:then_1
        (bind _outactors (Actor|GetAllActorsOfClass "/Script/Gear.GearPlayerState"))
        (for _array_element _outactors
          (bind _asgear_player_state (Utilities|Casting|CastToGearPlayerState _array_element))
          (CallFunction|NewPlayer _asgear_player_state))))))

(event EventOnAddPlayer
  (params (InPlayer :type Gear%20Player%20State%20Object%20Reference))
  (CallFunction|NewPlayer InPlayer))

(event EventOnRemovePlayer
  (params (InPlayer :type Gear%20Player%20State%20Object%20Reference))
  (CallFunction|RemovePlayer InPlayer))

(fn ConstructionScript)

(fn NewPlayer
  (params (Player :type Gear%20Player%20State%20Object%20Reference))
  (bind _waitingscreenwidget (Variables|Default|GetWaitingScreenWidget))
  (Utilities|IsValid _waitingscreenwidget
    (:Is%20Valid
      (Default|AddPlayer _waitingscreenwidget Player)
      (return))))

(fn RemovePlayer
  (params (NewParam :type Gear%20Player%20State%20Object%20Reference))
  (bind _waitingscreenwidget (Variables|Default|GetWaitingScreenWidget))
  (Utilities|IsValid _waitingscreenwidget
    (:Is%20Valid
      (Default|RemovePlayer _waitingscreenwidget NewParam)
      (return))))