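; BP_Fan_Test is a test fan actor that pushes an overlapping gear vehicle straight up along world Z.
; Begin overlap stores the BP_GearVehicle_Base reference and prints a debug string, and end overlap clears it for that same vehicle.
; While the reference is valid, Tick applies a large constant force to the vehicle's mesh, unscaled by mass, tracking only one vehicle at a time.
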(event EventBeginPlay)

(event Collision|EventActorBeginOverlap
  (params (OtherActor :type Actor%20Object%20Reference))
  (bind _asbp_gear_vehicle_base (Utilities|Casting|CastToBP_GearVehicle_Base OtherActor))
  (Variables|Default|SetAs%20BP%20Gear%20Vehicle%20Base _asbp_gear_vehicle_base)
  (Development|PrintString "Hello"))

(event EventTick
  (params (DeltaSeconds :type Float%20%28single-precision%29))
  (bind _as_bp_gear_vehicle_base (Variables|Default|GetAs%20BP%20Gear%20Vehicle%20Base)
    (:then
      (Physics|AddForce (Variables|/Script/ChaosVehicles.WheeledVehiclePawn|GetMesh _as_bp_gear_vehicle_base) "0.000000,0.000000,5000000.000000" "None" false))
    (:else)))

(event Collision|EventActorEndOverlap
  (params (OtherActor :type Actor%20Object%20Reference))
  (if (== OtherActor (Variables|Default|GetAs%20BP%20Gear%20Vehicle%20Base))
    (Variables|Default|SetAs%20BP%20Gear%20Vehicle%20Base 0)))

(fn ConstructionScript)